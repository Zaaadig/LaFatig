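; BP_Cube is a box the third-person character can push or pull while in its trigger and interacting.
; Box overlap events toggle CanInteractBox on the character reference cached at BeginPlay.
; Each Tick, if that flag and IsInteractingBox are set and the character moves, its forward/backward axis picks the direction.
; SpeedDirection interpolates the Cube's relative location, along its right vector for forward input and negative forward vector otherwise.
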(event OnComponentBeginOverlap(Box)
  (params (OverlappedComponent :type Primitive%20Component%20Object%20Reference) (OtherActor :type Actor%20Object%20Reference) (OtherComp :type Primitive%20Component%20Object%20Reference) (OtherBodyIndex :type Integer) (bFromSweep :type Boolean) (SweepResult :type Hit%20Result%20Structure%20%28by%20ref%29))
  (Development|PrintText "CanInteract" true true "(R=0.000000,G=0.660000,B=1.000000,A=1.000000)" 2.0 "159")
  (Variables|/Game/ThirdPerson/Blueprints/BP_ThirdPersonCharacter.BP_ThirdPersonCharacter_C|SetCanInteractBox? (Variables|Default|GetCharREF) true))

(event OnComponentEndOverlap(Box)
  (params (OverlappedComponent :type Primitive%20Component%20Object%20Reference) (OtherActor :type Actor%20Object%20Reference) (OtherComp :type Primitive%20Component%20Object%20Reference) (OtherBodyIndex :type Integer))
  (Development|PrintText "CannotInteract" true true "(R=1.000000,G=0.000000,B=0.041794,A=1.000000)" 2.0 "753")
  (Variables|/Game/ThirdPerson/Blueprints/BP_ThirdPersonCharacter.BP_ThirdPersonCharacter_C|SetCanInteractBox? (Variables|Default|GetCharREF) false))

(event EventBeginPlay
  (bind _returnvalue (Actor|GetActorOfClass "/Game/ThirdPerson/Blueprints/BP_ThirdPersonCharacter.BP_ThirdPersonCharacter_C"))
  (Variables|Default|SetCharREF _returnvalue))

(event Collision|EventActorBeginOverlap
  (params (OtherActor :type Actor%20Object%20Reference)))

(event EventTick
  (params (DeltaSeconds :type Float%20%28single-precision%29))
  (bind _charref (Variables|Default|GetCharREF))
  (bind _charref_2 (Variables|Default|GetCharREF))
  (if (Variables|/Game/ThirdPerson/Blueprints/BP_ThirdPersonCharacter.BP_ThirdPersonCharacter_C|GetIsInteractingBox? _charref)
    (if (Variables|/Game/ThirdPerson/Blueprints/BP_ThirdPersonCharacter.BP_ThirdPersonCharacter_C|GetCanInteractBox? _charref)
      (Utilities|FlowControl|Sequence
        (:then_0
          (if (Utilities|Operators|EqualEqual :A (Transformation|GetVelocity _charref_2))
            (Development|PrintString "idle" true true "(R=1.000000,G=0.016322,B=0.000000,A=1.000000)" 0.1 "198496")
            (elif (>= (Variables|/Game/ThirdPerson/Blueprints/BP_ThirdPersonCharacter.BP_ThirdPersonCharacter_C|GetForwardBackWardAxis _charref_2) 0.1)
              (Development|PrintString "Is Moving Forward" true true "(R=0.073642,G=1.000000,B=0.000000,A=1.000000)" 0.1 "1661")
              (Utilities|Speed/Direction true 6e+01)
              (else
                (Development|PrintString "Is Moving BackWards" true true "(R=0.073642,G=1.000000,B=0.000000,A=1.000000)" 0.1 "9955")
                (Utilities|Speed/Direction false -6e+01)))))))))

(fn ConstructionScript)