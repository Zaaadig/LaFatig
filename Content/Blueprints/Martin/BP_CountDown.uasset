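; BP_CountDown is a level countdown timer that kills the player and restarts the level when time runs out.
; It caches the BP_ThirdPersonCharacter on BeginPlay, then uses a one-second Delay on Tick to step Min and Sec down.
; At zero it prints a death message, calls RagdollTriggerMessage on the player, and reopens the current level by name after a short delay.
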(event EventBeginPlay
  (bind _returnvalue (Actor|GetActorOfClass "/Game/ThirdPerson/Blueprints/BP_ThirdPersonCharacter.BP_ThirdPersonCharacter_C"))
  (Variables|Default|SetPlayer _returnvalue))

(event EventTick
  (params (DeltaSeconds :type Float%20%28single-precision%29))
  (Utilities|FlowControl|Delay 1.0)
  ;[1 1 1] Timer ou le temps diminue progressivement
  (if (== (Variables|Default|GetSec) 0)
    (if (== (Variables|Default|GetMin) 0)
      ;[1 1 1] Animation de mort et Redémarrage de la scène si le conteur atteint 0
      (Development|PrintString "You Died Noob")
      (Class|BPITrap|RagdollTrigger(Message) (Variables|Default|GetPlayer))
      (Utilities|FlowControl|Delay 2.0)
      (bind _returnvalue (Game|GetCurrentLevelName true))
      (Game|OpenLevel(byName) (Utilities|String|StringToName _returnvalue))
      (else
        (Variables|Default|SetSec 59)
        (Variables|Default|SetMin (- (Variables|Default|GetMin) 1))))
    (else
      (Variables|Default|SetSec (- (Variables|Default|GetSec) 1)))))

(fn ConstructionScript)