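; BP_BOX is a pushable box that slides a set distance along the player's rounded forward direction when hit.
; CanPush line-traces from the player and box-traces the path, and the push runs when it returns false, despite the name.
; A Move timeline drives the slide while the player is attached with movement disabled, then restores walking.
; A separate overlap check against cached StaticMeshActors sets a CanPush flag.
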(event OnComponentBeginOverlap(Box)
  (params (OverlappedComponent :type Primitive%20Component%20Object%20Reference) (OtherActor :type Actor%20Object%20Reference) (OtherComp :type Primitive%20Component%20Object%20Reference) (OtherBodyIndex :type Integer) (bFromSweep :type Boolean) (SweepResult :type Hit%20Result%20Structure%20%28by%20ref%29))
  (bind _array_element (Utilities|Array|ForEachLoopwithBreak (Variables|Default|GetWalls) :!label _label)
    (:LoopBody
      (if (== _array_element OtherActor)
        (Variables|Default|SetCanPush false)
        (goto _label Break)
        (else
          (Variables|Default|SetCanPush true))))))

(event Custom|Push
  ;[1 1 1] Push + distance
  (Variables|Default|SetInitialLoc (Transformation|GetActorLocation))
  (bind _pos (Timeline|Move PlayFromStart)
    (:Update
      (Transformation|SetActorRelativeLocation (+ (Variables|Default|GetInitialLoc) (* _pos (Variables|Default|GetPushableDirection) (Variables|Default|GetTravelDistance)))))
    (:Finished
      (CallFunction|StopPush)
      (Development|PrintString "stop being pushed"))))

(event Custom|StopPush
  (bind _returnvalue (Game|GetPlayerCharacter 0))
  (Pawn|Components|CharacterMovement|SetMovementMode (Variables|/Script/Engine.Character|GetCharacterMovement _returnvalue) "MOVE_Walking" 0)
  (Transformation|DetachFromActor _returnvalue "KeepWorld" "KeepWorld" "KeepWorld")
  (Development|PrintString "detached"))

(event EventBeginPlay
  (bind _outactors (Actor|GetAllActorsOfClass "/Script/Engine.StaticMeshActor"))
  (Variables|Default|SetWalls _outactors))

(event Collision|EventHit
  (params (MyComp :type Primitive%20Component%20Object%20Reference) (Other :type Actor%20Object%20Reference) (OtherComp :type Primitive%20Component%20Object%20Reference) (bSelfMoved :type Boolean) (HitLocation :type Vector :default "0, 0, 0") (HitNormal :type Vector :default "0, 0, 0") (NormalImpulse :type Vector :default "0, 0, 0") (Hit :type Hit%20Result%20Structure%20%28by%20ref%29))
  (bind _returnvalue (Transformation|GetActorForwardVector Other))
  (bind _returnvalue_2 (Game|GetPlayerCharacter 0))
  (bind (_x _y _z) (Math|Vector|BreakVector _returnvalue))
  (if (== Other (Game|GetPlayerCharacter 0))
    (Variables|Default|SetPushableDirection (Math|Conversions|ToVector(Float) (Utilities|Struct|MakeIntVector (Math|Float|Round _x) (Math|Float|Round _y) (Math|Float|Round _z))))
    (bind _pushable (CallFunction|CanPush))
    (if (not _pushable)
      (Pawn|Components|CharacterMovement|DisableMovement (Variables|/Script/Engine.Character|GetCharacterMovement _returnvalue_2))
      (Transformation|AttachActorToActor _returnvalue_2 self "None" "KeepWorld" "KeepWorld" "KeepWorld" true)
      (CallFunction|Push))))

(fn ConstructionScript)

(fn CanPush
  (bind _returnvalue (Game|GetPlayerCharacter 0))
  (bind _returnvalue_2 (Transformation|GetActorLocation))
  (bind _cube (Variables|Default|GetCube))
  (bind _returnvalue_3 (Transformation|GetActorLocation _returnvalue))
  (bind _staticmesh (Variables|/Script/Engine.StaticMeshComponent|GetStaticMesh _cube))
  (bind _returnvalue_4 (StaticMesh|GetBounds _staticmesh))
  (bind (_outhit _returnvalue_5) (Collision|LineTraceByChannel _returnvalue_3 (+ _returnvalue_3 (* (Transformation|GetActorForwardVector _returnvalue) 1e+02)) "TraceTypeQuery1" false (Utilities|Array|MakeArray _returnvalue) "None" false))
  (if _returnvalue_5
    (if (== (.HitActor (Collision|BreakHitResult _outhit)) self)
      (bind _returnvalue_6 (Collision|BoxTraceByChannel (+ _returnvalue_2 (Math|Vector|MakeVector 0.0 0.0 1e+02)) (+ _returnvalue_2 (* (Variables|Default|GetPushableDirection) (Variables|Default|GetTravelDistance)) (.boxextent _returnvalue_4) (Math|Vector|MakeVector 0.0 0.0 1e+02)) (* (.boxextent _returnvalue_4) (Variables|/Script/Engine.SceneComponent|GetRelativeScale3D (Variables|Default|GetCube))) "0, 0, 0" "TraceTypeQuery1" false 0 "None"))
      (return (not _returnvalue_6))
      (else
        (return false)))
    (else
      (return false))))