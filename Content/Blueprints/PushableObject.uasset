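; Pushable block actor that slides a set distance when the player character walks into it head-on.
; On Hit, it rounds the player's forward vector into a push direction, and CanPush line-traces to confirm the player faces it, then box-traces the path for obstacles.
; During the push, the player's movement is disabled and they are attached to the block while a timeline moves it, then detached and restored to walking.
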(event Custom|Push
  (Variables|Default|SetCurrentLocation (Transformation|GetActorLocation))
  (bind _position (Timeline|MoveBlock PlayFromStart)
    (:Update
      (Transformation|SetActorRelativeLocation (+ (* _position (Variables|Default|GetPushableDirection) (Variables|Default|GetTravelDistance)) (Variables|Default|GetCurrentLocation))))
    (:Finished
      (CallFunction|StopPushing))))

(event Custom|StopPushing
  (bind _returnvalue (Game|GetPlayerCharacter 0))
  (Pawn|Components|CharacterMovement|SetMovementMode (Variables|/Script/Engine.Character|GetCharacterMovement _returnvalue) "MOVE_Walking" 0)
  (Transformation|DetachFromActor _returnvalue "KeepWorld" "KeepWorld" "KeepWorld"))

(event EventBeginPlay)

(event Collision|EventActorBeginOverlap
  (params (OtherActor :type Actor%20Object%20Reference)))

(event EventTick
  (params (DeltaSeconds :type Float%20%28single-precision%29)))

(event Collision|EventHit
  (params (MyComp :type Primitive%20Component%20Object%20Reference) (Other :type Actor%20Object%20Reference) (OtherComp :type Primitive%20Component%20Object%20Reference) (bSelfMoved :type Boolean) (HitLocation :type Vector :default "0, 0, 0") (HitNormal :type Vector :default "0, 0, 0") (NormalImpulse :type Vector :default "0, 0, 0") (Hit :type Hit%20Result%20Structure%20%28by%20ref%29))
  (bind _returnvalue (Transformation|GetActorForwardVector Other))
  (bind _returnvalue_2 (Game|GetPlayerCharacter 0))
  (bind (_x _y _z) (Math|Vector|BreakVector _returnvalue))
  (if (== (Game|GetPlayerCharacter 0) Other)
    (if (> (Math|Vector|DotProduct HitNormal _returnvalue) 0.93)
      (Variables|Default|SetPushableDirection (Math|Vector|MakeVector (Math|Conversions|ToFloat(Integer) (Math|Float|Round _x)) (Math|Conversions|ToFloat(Integer) (Math|Float|Round _y)) (Math|Conversions|ToFloat(Integer) (Math|Float|Round _z))))
      (bind _canpush (CallFunction|CanPush))
      (if _canpush
        (Pawn|Components|CharacterMovement|DisableMovement (Variables|/Script/Engine.Character|GetCharacterMovement _returnvalue_2))
        (Transformation|AttachActorToActor _returnvalue_2 self "None" "KeepWorld" "KeepWorld" "KeepWorld" true)
        (CallFunction|Push)))))

(fn ConstructionScript)

(fn CanPush
  (bind _returnvalue (Game|GetPlayerCharacter 0))
  (bind _returnvalue_2 (Transformation|GetActorLocation))
  (bind _returnvalue_3 (Transformation|GetActorLocation _returnvalue))
  (bind (_outhit _returnvalue_4) (Collision|LineTraceByChannel _returnvalue_3 (+ _returnvalue_3 (* (Transformation|GetActorForwardVector _returnvalue) 1e+02)) "TraceTypeQuery1" false (Utilities|Array|MakeArray _returnvalue) "None" false))
  (if _returnvalue_4
    (if (== (.HitActor (Collision|BreakHitResult _outhit)) self)
      (bind _returnvalue_5 (Collision|BoxTraceByChannel (+ _returnvalue_2 (Math|Vector|MakeVector 0.0 0.0 1e+02)) (+ _returnvalue_2 (* (Variables|Default|GetPushableDirection) (Variables|Default|GetTravelDistance)) (Math|Vector|MakeVector 0.0 0.0 1e+02)) (* (.boxextent (StaticMesh|GetBounds (Variables|/Script/Engine.StaticMeshComponent|GetStaticMesh (Variables|Default|GetCube)))) (Variables|/Script/Engine.SceneComponent|GetRelativeScale3D (Variables|Default|GetCube)) "0.900000,0.900000,0.900000") "0, 0, 0" "TraceTypeQuery1" false 0 "ForDuration"))
      (return (not _returnvalue_5))
      (else
        (return false)))
    (else
      (return false))))