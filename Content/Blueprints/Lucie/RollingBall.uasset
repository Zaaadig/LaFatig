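; Rolling ball hazard that moves along a path, ragdolls the player and restarts the level on contact.
; The construction script builds an InterpToMovement path from the ball's origin to a relative MoveToPos over a configurable Duration.
; Any ColliderBall overlap, with no actor check, ragdolls the character cached at BeginPlay, then reloads the current level after a short delay.
; Tag-check and teleport-to-start nodes remain unconnected.
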(event OnComponentBeginOverlap(ColliderBall)
  (params (OverlappedComponent :type Primitive%20Component%20Object%20Reference) (OtherActor :type Actor%20Object%20Reference) (OtherComp :type Primitive%20Component%20Object%20Reference) (OtherBodyIndex :type Integer) (bFromSweep :type Boolean) (SweepResult :type Hit%20Result%20Structure%20%28by%20ref%29))
  ;[0.3281 0 0.009124 0.588] Ragdoll
  (Class|BPITrap|RagdollTrigger(Message) (Variables|Default|GetPlayer))
  ;[0.1169 0.3958 0.07195 0.637] Respawn
  (Utilities|FlowControl|Delay 2.0)
  (bind _returnvalue (Game|GetCurrentLevelName true))
  (Game|OpenLevel(byName) (Utilities|String|StringToName _returnvalue)))

(event EventBeginPlay
  (bind _returnvalue (Actor|GetActorOfClass "/Game/ThirdPerson/Blueprints/BP_ThirdPersonCharacter.BP_ThirdPersonCharacter_C"))
  (Variables|Default|SetPlayer _returnvalue))

(event Collision|EventActorBeginOverlap
  (params (OtherActor :type Actor%20Object%20Reference)))

(event EventTick
  (params (DeltaSeconds :type Float%20%28single-precision%29)))

(fn ConstructionScript
  (bind _interptomovement (Variables|Default|GetInterpToMovement))
  (Class|InterptoMovementComponent|AddControlPointPosition (Variables|Default|GetInterpToMovement) "0, 0, 0" true)
  (Variables|/Script/Engine.InterpToMovementComponent|SetDuration _interptomovement (Variables|Default|GetDuration))
  (Class|InterptoMovementComponent|AddControlPointPosition _interptomovement (Variables|Default|GetMoveToPos) true))