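; BP_Cube is a box the third-person character can push, with debug prints of input and state.
; Fwd overlap events toggle the character's CanInteractBox flag.
; While that and IsInteractingBox are true, Tick reads the character's velocity and axes and calls SpeedDirection, which VInterps SMCube along its forward or right vector.
; Forward and backward pass the same positive speed, and sideways movement runs even without input.
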(event OnComponentBeginOverlap(Fwd)
  (params (OverlappedComponent :type Primitive%20Component%20Object%20Reference) (OtherActor :type Actor%20Object%20Reference) (OtherComp :type Primitive%20Component%20Object%20Reference) (OtherBodyIndex :type Integer) (bFromSweep :type Boolean) (SweepResult :type Hit%20Result%20Structure%20%28by%20ref%29))
  (Development|PrintString "Character Can Interact" true true "(R=0.066767,G=1.000000,B=0.000000,A=1.000000)" 2.0 "51513")
  (Variables|/Game/ThirdPerson/Blueprints/BP_ThirdPersonCharacter.BP_ThirdPersonCharacter_C|SetCanInteractBox? (Variables|Default|GetCharRef) true))

(event OnComponentEndOverlap(Fwd)
  (params (OverlappedComponent :type Primitive%20Component%20Object%20Reference) (OtherActor :type Actor%20Object%20Reference) (OtherComp :type Primitive%20Component%20Object%20Reference) (OtherBodyIndex :type Integer))
  (Development|PrintString "Character Can't Interact" true true "(R=1.000000,G=0.017360,B=0.000000,A=1.000000)" 2.0 "5616519")
  (Variables|/Game/ThirdPerson/Blueprints/BP_ThirdPersonCharacter.BP_ThirdPersonCharacter_C|SetCanInteractBox? (Variables|Default|GetCharRef) false))

(event EventBeginPlay
  (bind _returnvalue (Actor|GetActorOfClass "/Game/ThirdPerson/Blueprints/BP_ThirdPersonCharacter.BP_ThirdPersonCharacter_C"))
  (Variables|Default|SetCharRef _returnvalue))

(event EventTick
  (params (DeltaSeconds :type Float%20%28single-precision%29))
  (bind _charref (Variables|Default|GetCharRef))
  (bind _charref_2 (Variables|Default|GetCharRef))
  (bind _forwardbackwardsaxis (Variables|/Game/ThirdPerson/Blueprints/BP_ThirdPersonCharacter.BP_ThirdPersonCharacter_C|GetForwardBackwardsAxis _charref_2))
  (bind _rightleftaxis (Variables|/Game/ThirdPerson/Blueprints/BP_ThirdPersonCharacter.BP_ThirdPersonCharacter_C|GetRightLeftAxis _charref_2))
  (Development|PrintString (Utilities|String|ToString(Float) _forwardbackwardsaxis) true true "(R=1.000000,G=0.000000,B=0.966577,A=1.000000)")
  (Development|PrintString (Utilities|String|ToString(Float) _rightleftaxis) true true "(R=0.624124,G=0.000000,B=1.000000,A=1.000000)")
  (if (Variables|/Game/ThirdPerson/Blueprints/BP_ThirdPersonCharacter.BP_ThirdPersonCharacter_C|GetIsInteractingBox? _charref)
    (if (Variables|/Game/ThirdPerson/Blueprints/BP_ThirdPersonCharacter.BP_ThirdPersonCharacter_C|GetCanInteractBox? _charref)
      (Utilities|FlowControl|Sequence
        (:then_0
          (if (Utilities|Operators|EqualEqual :A (Transformation|GetVelocity _charref_2))
            (Development|PrintString "Player is not moving fwd or bkw" true true "(R=1.000000,G=0.036018,B=0.000000,A=1.000000)" 2.0 "646989")
            (elif (>= _forwardbackwardsaxis 0.1)
              (Development|PrintString "Is moving Forward" true true "(R=0.000000,G=0.820261,B=1.000000,A=1.000000)" 2.0 "269")
              (Utilities|Speed/Direction true 31.0)
              (else
                (Development|PrintString "Is Moving Backwards" true true "(R=0.000000,G=0.043959,B=1.000000,A=1.000000)" 2.0 "166764")
                (Utilities|Speed/Direction true 31.0)))))
        (:then_1
          (if (>= _rightleftaxis 0.1)
            (Development|PrintString "Is moving Right" true true "(R=0.000000,G=0.820261,B=1.000000,A=1.000000)" 2.0 "266519")
            (Utilities|Speed/Direction false -31.0)
            (else
              (Development|PrintString "Is Moving Left" true true "(R=0.000000,G=0.043959,B=1.000000,A=1.000000)" 2.0 "6597")
              (Utilities|Speed/Direction false 31.0))))))))

(fn ConstructionScript)